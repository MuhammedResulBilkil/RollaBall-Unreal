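; Base Blueprint for collectible items, extending a C++ parent that defines the Collected event.
; On the first collection only, it calls the parent's Collected logic, then multiplies the RotatingMovement rotation rate and InterpToMovement speed tenfold.
; The sped-up motion serves as pickup feedback for a short delay before the actor destroys itself.
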(event `self.Collected`
  (bind _rotatingmovement (`self.RotatingMovement`))
  (bind _interptomovement (`self.InterpToMovement`))
  (`/Engine/EditorBlueprintResources/StandardMacros.DoOnce` false
    (:`Completed`
      (`parent.Collected`) ; This makes call the C++ side of this call
      (set `RotatingMovementComponent.RotationRate` (* (`RotatingMovementComponent.RotationRate` _rotatingmovement) 10.0) _rotatingmovement)
      (set `InterpToMovementComponent.SpeedMultiplier` (* (`InterpToMovementComponent.SpeedMultiplier` _interptomovement) 10.0) _interptomovement)
      (`KismetSystemLibrary.Delay` 2.0)
      (`self.K2_DestroyActor`))))

(fn `UserConstructionScript`)